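; Dog companion pawn that exposes Stay/Roam, Follow and MovetoTarget commands for its AI.
; On BeginPlay it caches its AIC_Dog_Companion controller, and each command forwards a companion state plus any follow actor or target location to it.
; Follow also plays a bark through an immediately reset DoOnce.
; Obey/Disobey is empty, with its random-choice logic left disconnected.
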(event `self.ReceiveBeginPlay`
  (bind _asaic_dog_companion (cast `/Game/AI/AI_Dog_Companion/AIC_Dog_Companion` (`AIBlueprintHelperLibrary.GetAIController` self)))
  (set `self.Companion Controller` _asaic_dog_companion))

(event `Stay/Roam`
  (`/Game/AI/AI_Dog_Companion/AIC_Dog_Companion.SetCompanionState` (`self.Companion Controller`) "NewEnumerator0")
  (`/Game/AI/AI_Dog_Companion/AIC_Dog_Companion.SetCompanionState` (`self.Companion Controller`) "NewEnumerator3"))

(event `Follow`
  (params (`Follow Target` :type "Actor Object Reference"))
  (bind _companion_controller (`self.Companion Controller`))
  (`/Game/AI/AI_Dog_Companion/AIC_Dog_Companion.SetFollowActor` _companion_controller `Follow Target`)
  (`/Game/AI/AI_Dog_Companion/AIC_Dog_Companion.SetCompanionState` _companion_controller "NewEnumerator1")
  (`/Engine/EditorBlueprintResources/StandardMacros.DoOnce` false :!label _label
    (:`Completed`
      (`GameplayStatics.PlaySoundAtLocation` "/Game/AI/AI_Dog_Companion/Dog_Sounds/4912__noisecollector__barks.4912__noisecollector__barks" (`self.K2_GetActorLocation`) (struct) 1.0 1.0 0.0 null null null null)
      (goto _label :!via `Reset`))))

(event `Move to Target`
  (params (Location :type "Vector Structure"))
  (`/Game/AI/AI_Dog_Companion/AIC_Dog_Companion.SetTargetLocation` (`self.Companion Controller`) Location)
  (`/Game/AI/AI_Dog_Companion/AIC_Dog_Companion.SetCompanionState` (`self.Companion Controller`) "NewEnumerator2"))

(event `Obey/Disobey`)

(event `self.ReceiveTick`
  (params (DeltaSeconds :type "Float (single-precision)")))

(fn `UserConstructionScript`)