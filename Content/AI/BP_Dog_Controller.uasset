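; BP_Dog_Controller is the AI controller for a dog character driven by the BT_Dog behavior tree.
; On BeginPlay it starts that tree, provided the controlled pawn is a BP_Placeholder_AI.
; Its CallDog, GiveCommand and DoThing events each set a matching Blackboard bool to true, and nothing here resets those flags.
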(event `self.ReceiveBeginPlay`
  (cast `/Game/AI/BP_Placeholder_AI` (`self.K2_GetPawn`))
  (`self.RunBehaviorTree` "/Game/AI/BT_Dog.BT_Dog"))

(event `Call  Dog`
  (`BlackboardComponent.SetValueAsBool` (`AIBlueprintHelperLibrary.GetBlackboard` null) "Call Dog" true))

(event `Give Command`
  (`BlackboardComponent.SetValueAsBool` (`AIBlueprintHelperLibrary.GetBlackboard` null) "Given Command" true))

(event `Do Thing`
  (`BlackboardComponent.SetValueAsBool` (`AIBlueprintHelperLibrary.GetBlackboard` null) "DO Thing" true))

(fn `UserConstructionScript`)