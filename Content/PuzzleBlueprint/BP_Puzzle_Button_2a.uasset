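; Three-button pressure plate puzzle in which overlapping each plate's box toggles that button on or off.
; While the puzzle is active and unsolved, each toggle updates that button's light and material, plays a beep and checks whether all three are on.
; When all are on, it locks as solved, applies finished colours and materials, plays a bell and calls PuzzleSolveFunction on BP_Puzzle_Master.
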(event `self.ReceiveBeginPlay`
  (`parent.ReceiveBeginPlay`)
  (`LightComponent.SetLightColor` (`self.A_PointLight1`) (`self.Off Colour`) true)
  (`LightComponent.SetLightColor` (`self.B_PointLight`) (`self.Off Colour`) true)
  (`LightComponent.SetLightColor` (`self.C_PointLight1`) (`self.Off Colour`) true)
  (`LightComponent.SetLightColor` (`self.A_PointLight1`) (`self.Off Colour`) true))

(event `self.A_Box2.OnComponentBeginOverlap`
  (params (OverlappedComponent :type "PrimitiveComponent Object Reference") (OtherActor :type "Actor Object Reference") (OtherComp :type "PrimitiveComponent Object Reference") (OtherBodyIndex :type Integer) (bFromSweep :type Boolean) (SweepResult :type "HitResult Structure (by ref)"))
  (bind _output (`|GetArrayItem` (`self.Is On`)))
  ;[1 1 1] Individual pressure plate toggles
  (if (and (`self.IsActive`) (!= (`self.Is Solved`) true))
    (if _output
      (`KismetArrayLibrary.Array_Set` (`self.Is On`))
      (else
        (`KismetArrayLibrary.Array_Set` (`self.Is On`) 0 true)))
    (`self.Update Light` (`self.A_PointLight1`) _output)
    (bind _isfullyactive (`self.FullyActiveCheck` :!label _label))
    (`GameplayStatics.PlaySoundAtLocation` "/Game/PuzzleSounds/Button_beep.Button_beep" (`self.K2_GetActorLocation` (`GameplayStatics.GetPlayerCharacter` 0)) (struct) 1.0 1.0 0.0 null null null null)
    (if _isfullyactive
      (`self.End Process`)
      (`GameplayStatics.PlaySoundAtLocation` "/Game/PuzzleSounds/Success_Bell.Success_Bell" (`self.K2_GetActorLocation` (`GameplayStatics.GetPlayerCharacter` 0)) (struct) 1.0 1.0 0.0 null null null null)
      (else
        (for _ (`self.Is On`)
          _)))))

(event `self.B_Box.OnComponentBeginOverlap`
  (params (OverlappedComponent :type "PrimitiveComponent Object Reference") (OtherActor :type "Actor Object Reference") (OtherComp :type "PrimitiveComponent Object Reference") (OtherBodyIndex :type Integer) (bFromSweep :type Boolean) (SweepResult :type "HitResult Structure (by ref)"))
  (bind _output (`|GetArrayItem` (`self.Is On`) 1))
  ;[1 1 1] Individual pressure plate toggles
  (if (and (`self.IsActive`) (!= (`self.Is Solved`) true))
    (if _output
      (`KismetArrayLibrary.Array_Set` (`self.Is On`) 1)
      (else
        (`KismetArrayLibrary.Array_Set` (`self.Is On`) 1 true)))
    (`self.Update Light` (`self.B_PointLight`) _output 1)
    (goto _label)))

(event `End Process`
  (set `self.Is Solved` true)
  (`LightComponent.SetLightColor` (`self.A_PointLight1`) (`self.Solved Colour`) true)
  (`LightComponent.SetLightColor` (`self.B_PointLight`) (`self.Solved Colour`) true)
  (`LightComponent.SetLightColor` (`self.C_PointLight1`) (`self.Solved Colour`) true)
  (`PrimitiveComponent.SetMaterial` (`self.A_Button`) 0 (`self.Mat_Finished`))
  (`PrimitiveComponent.SetMaterial` (`self.B_Button`) 0 (`self.Mat_Finished`))
  (`PrimitiveComponent.SetMaterial` (`self.C_Button`) 0 (`self.Mat_Finished`))
  (bind _asbp_puzzle_master (cast `/Game/PuzzleBlueprint/BP_Puzzle_Master` (`self.Puzzle_Master_Reference`)))
  (`/Game/PuzzleBlueprint/BP_Puzzle_Master.Puzzle Solve Function` _asbp_puzzle_master 1))

(event `self.C_Box1.OnComponentBeginOverlap`
  (params (OverlappedComponent :type "PrimitiveComponent Object Reference") (OtherActor :type "Actor Object Reference") (OtherComp :type "PrimitiveComponent Object Reference") (OtherBodyIndex :type Integer) (bFromSweep :type Boolean) (SweepResult :type "HitResult Structure (by ref)"))
  (bind _output (`|GetArrayItem` (`self.Is On`) 2))
  ;[1 1 1] Individual pressure plate toggles
  (if (and (`self.IsActive`) (!= (`self.Is Solved`) true))
    (if _output
      (`KismetArrayLibrary.Array_Set` (`self.Is On`) 2)
      (else
        (`KismetArrayLibrary.Array_Set` (`self.Is On`) 2 true)))
    (`self.Update Light` (`self.C_PointLight1`) _output 2)
    (goto _label)))

(fn `FullyActiveCheck`
  (returns (IsFullyActive :type Boolean))
  (bind _is_on (`self.Is On`))
  (bind _returnvalue (and (and (`|GetArrayItem` _is_on) (`|GetArrayItem` _is_on 1)) (`|GetArrayItem` _is_on 2)))
  (if (not _returnvalue)
    (`KismetSystemLibrary.PrintString` "Nothing happens"))
  (return _returnvalue))

(fn `Update Light`
  (params (`Taget Light` :type "PointLightComponent Object Reference") (`Is Active` :type Boolean) (`Target Index` :type Integer))
  (`LightComponent.SetLightColor` (select `int` `Target Index` :`0` (`self.A_PointLight1`) :`1` (`self.B_PointLight`) :`2` (`self.C_PointLight1`)) (select `bool` `Is Active` :`false` (`self.Off Colour`) :`true` (`self.On Colour`)) true)
  (`PrimitiveComponent.SetMaterial` (select `int` `Target Index` :`0` (`self.A_Button`) :`1` (`self.B_Button`) :`2` (`self.C_Button`)) 0 (select `bool` `Is Active` :`false` (`self.Mat_Inactive`) :`true` (`self.Mat_Active`))))

(fn `UserConstructionScript`
  (`parent.UserConstructionScript`))