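; Combination puzzle Blueprint with four drums, each cycling through four positions and represented by a colored point light as a placeholder visual.
; BeginPlay randomizes every drum, rerolling any value that matches its solution digit so the puzzle cannot start solved.
; ObjectInteract advances the indexed drum with wraparound, runs SolvedCheck against the solution array and recolors a light through UpdateLight.
; Solving currently only prints debug messages.
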(event `self.ReceiveBeginPlay`
  (`self.Randomise Start`))

(event `/Game/PuzzleBlueprint/BPI_Puzzle_Interact.Object Interact`
  (params (TargetIndex :type Integer))
  (bind _drum_position_array (`self.Drum_Position_Array`))
  (bind _returnvalue (mod (+ (`|GetArrayItem` _drum_position_array TargetIndex) 1) 4))
  ;[0.04774 1 0.0511] Properly funcitoning code
  (`KismetArrayLibrary.Array_Set` _drum_position_array TargetIndex _returnvalue)
  (`self.Solved Check`)
  ;[1 0 0.2471] Visual element (TO BE REPLACED
  (`self.UpdateLight` (select `int` TargetIndex :`0` (`self.A_PointLight`) :`1` (`self.B_PointLight`) :`2` (`self.C_PointLight`) :`3` (`self.D_PointLight`)) _returnvalue)
  ;[1 0.268 0] debug
  (for _array_element (`self.Drum_Position_Array`)
    (`KismetSystemLibrary.PrintString` (`KismetStringLibrary.Conv_IntToString` _array_element))))

(event `Randomise Start`
  ;[1 0.666 0.03035] Randomise combination at start
  (for _index (range 4)
    ;;[1 1 1] Prevents self-solving
    (bind _output_get (set `self.Temp Value` (`KismetMathLibrary.RandomIntegerInRange` 0 3) :!label _label))
    (if (== _output_get (`|GetArrayItem` (`self.Solution_Position_Array`) _index))
      (goto _label)
      (else
        (`KismetArrayLibrary.Array_Set` (`self.Drum_Position_Array`) _index (`self.Temp Value`))
        ;[1 0 0.1436] Visual Element (TO BE REPLACED
        (`LightComponent.SetLightColor` (select `int` _index :`0` (`self.A_PointLight`) :`1` (`self.B_PointLight`) :`2` (`self.C_PointLight`) :`3` (`self.D_PointLight`)) (select `int` (`self.Temp Value`) :`0` (`self.Light Colour_0`) :`1` (`self.Light Colour_1`) :`2` (`self.Light Colour_2`) :`3` (`self.Light Colour_3`)) true)))))

(event `Solved Check`
  ;[0.3132 1 0] Check for solution
  (`KismetSystemLibrary.PrintString` "Solved Check start" true true (struct :`R` 1.0 :`G` 0.544528 :`B` 0.11876 :`A` 1.0))
  (set `self.Temp_SolvedBool` true)
  (for (_array_element _array_index) (`self.Drum_Position_Array`)
    (if (not (== _array_element (`|GetArrayItem` (`self.Solution_Position_Array`) _array_index)))
      (set `self.Temp_SolvedBool` false)))
  (if (`self.Temp_SolvedBool`)
    (`KismetSystemLibrary.PrintString` "Puzzle Solved" true true (struct :`R` 1.0 :`G` 0.464126 :`A` 1.0) 5.0)
    (else
      (`KismetSystemLibrary.PrintString` "Puzzzle Unsolved"))))

(fn `NewFunction_0`)

(fn `UpdateLight`
  (params (LightObject :type "PointLightComponent Object Reference") (Value :type Integer))
  (`LightComponent.SetLightColor` LightObject (select `int` Value :`0` (`self.Light Colour_0`) :`1` (`self.Light Colour_1`) :`2` (`self.Light Colour_2`) :`3` (`self.Light Colour_3`)) true))

(fn `UserConstructionScript`
  (`parent.UserConstructionScript`))