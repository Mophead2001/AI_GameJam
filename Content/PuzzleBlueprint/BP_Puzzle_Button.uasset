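; BP_Puzzle_Button is a puzzle button that triggers a linked Target object when anything begins overlapping its Box.
; The overlap calls ButtonActivate, which prints debug text and sends ObjectInteractMessage to Target with TargetIndex.
; The Button then briefly flashes its active material before reverting to inactive after a short Delay.
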(event `ButtonActivate`
  (bind _targetindex (`self.TargetIndex`))
  (`KismetSystemLibrary.PrintString` "ButtonActivate")
  (`KismetSystemLibrary.PrintString` (`KismetStringLibrary.Conv_IntToString` _targetindex) true true (struct :`R` 0.471072 :`G` 1.0 :`A` 1.0))
  (message `/Game/PuzzleBlueprint/BPI_Puzzle_Interact.Object Interact` (`self.Target`) _targetindex))

(event `self.Box.OnComponentBeginOverlap`
  (params (OverlappedComponent :type "PrimitiveComponent Object Reference") (OtherActor :type "Actor Object Reference") (OtherComp :type "PrimitiveComponent Object Reference") (OtherBodyIndex :type Integer) (bFromSweep :type Boolean) (SweepResult :type "HitResult Structure (by ref)"))
  (`self.ButtonActivate`)
  (`PrimitiveComponent.SetMaterial` (`self.Button`) 0 (`self.Mat_Active`))
  (`KismetSystemLibrary.Delay` 0.2)
  (`PrimitiveComponent.SetMaterial` (`self.Button`) 0 (`self.Mat_Inactive`)))

(fn `UserConstructionScript`)