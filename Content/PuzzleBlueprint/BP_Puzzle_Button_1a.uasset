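; Puzzle pressure button that must stay overlapped until its progress fills, then reports solved to the puzzle master with index 0.
; Box overlaps toggle active and inactive states, switching light colour, button material and the sign of the progress rate.
; Tick accumulates clamped progress per frame without delta time, so it drains when released and fill speed depends on framerate.
; On completion it locks into a finished look and closes the Tick gate.
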(event `self.ReceiveBeginPlay`
  (`self.Puzzle Deactivate`))

(event `self.ReceiveTick`
  (params (DeltaSeconds :type "Float (single-precision)"))
  (`/Engine/EditorBlueprintResources/StandardMacros.Gate` false :!label _label
    (:`Exit`
      (bind _output_get (set `self.ProgressFloat` (`KismetMathLibrary.FClamp` (+ (`self.ProgressFloat`) (`self.ProgressCoefficient`)) 0.0 1.1)))
      (if (>= _output_get 1.0)
        (`/Game/PuzzleBlueprint/BP_Puzzle_Master.Puzzle Solve Function` (`self.BP_PuzzleMaster_Ref`) 0)
        (`self.Puzzle Finish`)
        (goto _label :!via `Close`)))))

(event `self.Box.OnComponentBeginOverlap`
  (params (OverlappedComponent :type "PrimitiveComponent Object Reference") (OtherActor :type "Actor Object Reference") (OtherComp :type "PrimitiveComponent Object Reference") (OtherBodyIndex :type Integer) (bFromSweep :type Boolean) (SweepResult :type "HitResult Structure (by ref)"))
  (if (not (`self.Is Solved`))
    (`self.Puzzle Activate`)))

(event `Puzzle Activate`
  (`LightComponent.SetLightColor` (`self.PointLight`) (`self.ActiveColour`) true)
  (`PrimitiveComponent.SetMaterial` (`self.Button`) 0 (`self.Mat_Active`))
  (set `self.ProgressCoefficient` 0.01))

(event `Puzzle Deactivate`
  (`LightComponent.SetLightColor` (`self.PointLight`) (`self.Inactive Colour`) true)
  (`PrimitiveComponent.SetMaterial` (`self.Button`) 0 (`self.Mat_Inactive`))
  (set `self.ProgressCoefficient` -0.01))

(event `self.Box.OnComponentEndOverlap`
  (params (OverlappedComponent :type "PrimitiveComponent Object Reference") (OtherActor :type "Actor Object Reference") (OtherComp :type "PrimitiveComponent Object Reference") (OtherBodyIndex :type Integer))
  (if (not (`self.Is Solved`))
    (`self.Puzzle DeActivate`)))

(event `Puzzle Finish`
  (set `self.Is Solved` true)
  (`LightComponent.SetLightColor` (`self.PointLight`) (`self.Finished Light Colour`) true)
  (`PrimitiveComponent.SetMaterial` (`self.Button`) 0 (`self.Mat_Finished`)))

(fn `UserConstructionScript`
  (`parent.UserConstructionScript`))