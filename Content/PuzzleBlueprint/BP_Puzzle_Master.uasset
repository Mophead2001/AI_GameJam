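; BP_Puzzle_Master tracks completion of three puzzles and signals a door unlock once all are solved.
; PuzzleSolveFunction prints the solved index, sets that entry in IsPuzzleCompleteArray and calls AllSolvedCheck.
; AllSolvedCheck tests the first three array entries, prints a message and calls UnlockDoor, which is an empty stub.
; The PuzzleSolved_1 event is also empty, with a disconnected copy of the solve logic left in the event graph.
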(event `Puzzle Solved_1`
  (params (`Puzzle Index` :type Integer)))

(event `All Solved Check`
  (bind _ispuzzlecompletearray (`self.IsPuzzleCompleteArray`))
  (if (and (and (`|GetArrayItem` _ispuzzlecompletearray) (`|GetArrayItem` _ispuzzlecompletearray 1)) (`|GetArrayItem` _ispuzzlecompletearray 2))
    (`KismetSystemLibrary.PrintString` "ALL PUZZLES SOLVED")
    (`self.Unlock Door`)))

(event `Unlock Door`)

(fn `Puzzle Solve Function`
  (params (NewParam :type Integer))
  (`KismetSystemLibrary.PrintString` (`KismetStringLibrary.Conv_IntToString` NewParam) true true (struct :`R` 1.0 :`G` 0.631885 :`A` 1.0))
  (`KismetSystemLibrary.PrintString` "Is solved" true true (struct :`R` 1.0 :`G` 0.015156 :`A` 1.0))
  (`KismetArrayLibrary.Array_Set` (`self.IsPuzzleCompleteArray`) NewParam true)
  (`self.All Solved Check`))

(fn `UserConstructionScript`)