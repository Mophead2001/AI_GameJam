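; BP_BunkerDoor is a puzzle bunker door that swings open when its Open event is called.
; Open captures the root's world transform, then a timeline interpolates only the rotation toward EndTransform, keeping location and scale fixed.
; A DoOnce on the timeline update plays the door-opening sound a single time, at the player character's location rather than the door's.
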(event `self.ReceiveBeginPlay`)

(event `Open`
  (bind (_starttransform_location _starttransform_rotation _starttransform_scale) (`KismetMathLibrary.BreakTransform` (`self.StartTransform`)))
  (bind (_endtransform_location _endtransform_rotation) (`KismetMathLibrary.BreakTransform` (`self.EndTransform`)))
  (set `self.StartTransform` (`SceneComponent.K2_GetComponentToWorld` (`self.DefaultSceneRoot`)))
  (bind (_direction _opentrack) (`Timeline|OpenDoorTimeline` :!via `PlayFromStart`)
    (:`Update`
      (`SceneComponent.K2_SetWorldTransform` (`self.DefaultSceneRoot`) (`KismetMathLibrary.TLerp` (`KismetMathLibrary.MakeTransform` _starttransform_location _starttransform_rotation _starttransform_scale) (`KismetMathLibrary.MakeTransform` _starttransform_location _endtransform_rotation _starttransform_scale) _opentrack) false false)
      (`/Engine/EditorBlueprintResources/StandardMacros.DoOnce` false
        (:`Completed`
          (`GameplayStatics.PlaySoundAtLocation` "/Game/PuzzleSounds/Door_Opening.Door_Opening" (`self.K2_GetActorLocation` (`GameplayStatics.GetPlayerCharacter` 0)) (struct) 1.0 1.0 0.0 null null null null))))))

(fn `UserConstructionScript`)