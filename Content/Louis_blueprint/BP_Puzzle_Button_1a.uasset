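; BP_Puzzle_Button_1a is a puzzle button actor that shows whether something is standing in its trigger.
; Box overlap begin fires PuzzleActivate and overlap end fires PuzzleDeactivate, each recolouring a PointLight to the active or inactive colour.
; BeginPlay deactivates it, and overlaps are not filtered by actor or counted, so any exiting component switches it off.
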(event `self.ReceiveBeginPlay`
  (`self.Puzzle Deactivate`))

(event `self.Box.OnComponentBeginOverlap`
  (params (OverlappedComponent :type "PrimitiveComponent Object Reference") (OtherActor :type "Actor Object Reference") (OtherComp :type "PrimitiveComponent Object Reference") (OtherBodyIndex :type Integer) (bFromSweep :type Boolean) (SweepResult :type "HitResult Structure (by ref)"))
  (`self.Puzzle Activate`))

(event `Puzzle Activate`
  (`LightComponent.SetLightColor` (`self.PointLight`) (`self.ActiveColour`) true))

(event `self.Box.OnComponentEndOverlap`
  (params (OverlappedComponent :type "PrimitiveComponent Object Reference") (OtherActor :type "Actor Object Reference") (OtherComp :type "PrimitiveComponent Object Reference") (OtherBodyIndex :type Integer))
  (`self.Puzzle DeActivate`))

(event `Puzzle Deactivate`
  (`LightComponent.SetLightColor` (`self.PointLight`) (`self.Inactive Colour`) true))

(fn `UserConstructionScript`
  (`parent.UserConstructionScript`))