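; BP_Puzzle_Combination is a combination puzzle with four drum positions, each paired with a point light.
; ObjectInteract advances the targeted DrumPositionArray entry, wrapping after four states, and prints a debug string.
; It then recolours that drum's light from four colours, recomputing the increment from the already updated entry.
; An UpdateLight helper duplicates the colour selection but is not called here, and no solution check is present.
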(event `/Game/Louis_blueprint/BPI_Puzzle_Interact.Object Interact`
  (params (TargetIndex :type Integer))
  (bind _drum_position_array (`self.Drum_Position_Array`))
  (bind _returnvalue (mod (+ (`|GetArrayItem` _drum_position_array TargetIndex) 1) 4))
  (`KismetSystemLibrary.PrintString` "Successfulcast")
  (`KismetArrayLibrary.Array_Set` _drum_position_array TargetIndex _returnvalue)
  (`LightComponent.SetLightColor` (select `int` TargetIndex :`0` (`self.A_PointLight`) :`1` (`self.B_PointLight`) :`2` (`self.C_PointLight`) :`3` (`self.D_PointLight`)) (select `int` _returnvalue :`0` (`self.Light Colour_1`) :`1` (`self.Light Colour_2`) :`2` (`self.Light Colour_3`) :`3` (`self.Light Colour_4`)) true))

(fn `UpdateLight`
  (params (LightObject :type "PointLightComponent Object Reference") (PositionIndex :type Integer))
  (`LightComponent.SetLightColor` LightObject (select `int` PositionIndex :`0` (`self.Light Colour_1`) :`1` (`self.Light Colour_2`) :`2` (`self.Light Colour_3`) :`3` (`self.Light Colour_4`)) true))

(fn `UserConstructionScript`
  (`parent.UserConstructionScript`))