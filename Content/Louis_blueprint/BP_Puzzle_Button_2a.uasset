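; BP_Puzzle_Button_2a is a puzzle actor with three pressure plates, solved when all three are active at once.
; Each box overlap toggles its entry in a boolean array and recolours the matching point light to the active or inactive colour.
; A shared check then tests all three entries and prints a debug string.
; On success it sets IsSolved, which blocks further toggling, and turns every light cyan.
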(event `self.ReceiveBeginPlay`
  (`parent.ReceiveBeginPlay`)
  (`LightComponent.SetLightColor` (`self.A_PointLight2`) (`self.Inactive Colour`) true)
  (`LightComponent.SetLightColor` (`self.B_PointLight`) (`self.Inactive Colour`) true)
  (`LightComponent.SetLightColor` (`self.C_PointLight1`) (`self.Inactive Colour`) true))

(event `self.A_Box2.OnComponentBeginOverlap`
  (params (OverlappedComponent :type "PrimitiveComponent Object Reference") (OtherActor :type "Actor Object Reference") (OtherComp :type "PrimitiveComponent Object Reference") (OtherBodyIndex :type Integer) (bFromSweep :type Boolean) (SweepResult :type "HitResult Structure (by ref)"))
  (bind _output (`|GetArrayItem` (`self.IsActiveBoolean`)))
  ;[1 1 1] Individual pressure plate toggles
  (if (not (`self.IsSolved`))
    (if _output
      (`KismetArrayLibrary.Array_Set` (`self.IsActiveBoolean`))
      (else
        (`KismetArrayLibrary.Array_Set` (`self.IsActiveBoolean`) 0 true)))
    (`self.Update Light` (`self.A_PointLight2`) _output)
    (bind _isfullyactive (`self.FullyActiveCheck` :!label _label))
    (if _isfullyactive
      (`self.End Process`))))

(event `self.B_Box.OnComponentBeginOverlap`
  (params (OverlappedComponent :type "PrimitiveComponent Object Reference") (OtherActor :type "Actor Object Reference") (OtherComp :type "PrimitiveComponent Object Reference") (OtherBodyIndex :type Integer) (bFromSweep :type Boolean) (SweepResult :type "HitResult Structure (by ref)"))
  (bind _output (`|GetArrayItem` (`self.IsActiveBoolean`) 1))
  ;[1 1 1] Individual pressure plate toggles
  (if (not (`self.IsSolved`))
    (if _output
      (`KismetArrayLibrary.Array_Set` (`self.IsActiveBoolean`) 1)
      (else
        (`KismetArrayLibrary.Array_Set` (`self.IsActiveBoolean`) 1 true)))
    (`self.Update Light` (`self.B_PointLight`) _output)
    (goto _label)))

(event `End Process`
  (set `self.IsSolved` true)
  (`LightComponent.SetLightColor` (`self.A_PointLight2`) (struct :`G` 0.909328 :`B` 1.0 :`A` 1.0) true)
  (`LightComponent.SetLightColor` (`self.B_PointLight`) (struct :`G` 0.909328 :`B` 1.0 :`A` 1.0) true)
  (`LightComponent.SetLightColor` (`self.C_PointLight1`) (struct :`G` 0.909328 :`B` 1.0 :`A` 1.0) true))

(event `self.C_Box1.OnComponentBeginOverlap`
  (params (OverlappedComponent :type "PrimitiveComponent Object Reference") (OtherActor :type "Actor Object Reference") (OtherComp :type "PrimitiveComponent Object Reference") (OtherBodyIndex :type Integer) (bFromSweep :type Boolean) (SweepResult :type "HitResult Structure (by ref)"))
  (bind _output (`|GetArrayItem` (`self.IsActiveBoolean`) 2))
  ;[1 1 1] Individual pressure plate toggles
  (if (not (`self.IsSolved`))
    (if _output
      (`KismetArrayLibrary.Array_Set` (`self.IsActiveBoolean`) 2)
      (else
        (`KismetArrayLibrary.Array_Set` (`self.IsActiveBoolean`) 2 true)))
    (`self.Update Light` (`self.C_PointLight1`) _output)
    (goto _label)))

(fn `FullyActiveCheck`
  (returns (IsFullyActive :type Boolean))
  (bind _isactiveboolean (`self.IsActiveBoolean`))
  (bind _returnvalue (and (and (`|GetArrayItem` _isactiveboolean) (`|GetArrayItem` _isactiveboolean 1)) (`|GetArrayItem` _isactiveboolean 2)))
  (if _returnvalue
    (`KismetSystemLibrary.PrintString` "Activate")
    (else
      (`KismetSystemLibrary.PrintString` "Nothing happens")))
  (return _returnvalue))

(fn `Update Light`
  (params (NewParam :type "PointLightComponent Object Reference") (`Is Active` :type Boolean))
  (`LightComponent.SetLightColor` NewParam (select `bool` `Is Active` :`false` (`self.Inactive Colour`) :`true` (`self.Active Colour`)) true))

(fn `UserConstructionScript`
  (`parent.UserConstructionScript`))